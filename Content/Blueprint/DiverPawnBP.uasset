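; DiverPawnBP is a diver pawn that pairs a VR pawn component with a mannequin body and handles dive controls.
; On BeginPlay it enables input through player 0's controller and attaches VRPawn to the mannequin's head socket, so it follows the head.
; The StartDive and ComeOut input actions each set a flag to true and pass it out through their matching event calls.
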(event Input|EnhancedActionEvents|EnhancedInputActionStartDiveEvent
  (params (ActionValue :type Boolean) (ElapsedSeconds :type Float%20%28double-precision%29) (TriggeredSeconds :type Float%20%28double-precision%29) (InputAction :type Input%20Action%20Object%20Reference :default "/Game/Input/StartDiveEvent.StartDiveEvent"))
  (:Started
    (bind _output_get (Variables|Default|SetStartDive true))
    (Default|CallStartDiveEvent _output_get)))

(event Input|EnhancedActionEvents|EnhancedInputActionComeOutEvent
  (params (ActionValue :type Boolean) (ElapsedSeconds :type Float%20%28double-precision%29) (TriggeredSeconds :type Float%20%28double-precision%29) (InputAction :type Input%20Action%20Object%20Reference :default "/Game/Input/ComeOutEvent.ComeOutEvent"))
  (:Started
    (bind _output_get (Variables|Default|SetComeOut true))
    (Default|CallComeOutEvent _output_get)))

(event EventBeginPlay
  (Input|EnableInput (Game|GetPlayerController (Variables|/Script/Engine.Pawn|GetPlayerState (Game|Player|GetPlayerPawn 0))))
  (Transformation|AttachComponentToComponent (Variables|Default|GetVRPawn) (Variables|Default|GetSK_Mannequin) "headSocket" "KeepRelative" "KeepRelative" "KeepRelative" true))

(fn ConstructionScript)