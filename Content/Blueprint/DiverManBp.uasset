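; DiverManBp is a diver actor that plays a starting animation and can spin around a center-of-mass component.
; BeginPlay enables input; G stores the CenterOfMass world rotation, plays the starting sequence once on the mannequin and sets a started flag.
; P prints a debug string and toggles rotation through a FlipFlop.
; Once started, Tick increments roll by a fixed step per frame while rotation is on, independent of delta time.
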(event Collision|EventActorBeginOverlap
  (params (OtherActor :type Actor%20Object%20Reference)))

(event EventTick
  (params (DeltaSeconds :type Float%20%28single-precision%29))
  (if (Variables|Default|GetisStartingAnimPlayed?)
    (if (Variables|Default|GetRoation)
      (bind _output_get (Variables|Default|SetInitialRotation (Math|Rotator|MakeRotator (+ (.roll (Variables|Default|GetInitialRotation)) 1.0) (.pitch (Variables|Default|GetInitialRotation)) (.yaw (Variables|Default|GetInitialRotation)))))
      (Transformation|SetWorldRotation (Variables|Default|GetCenterOfMass) _output_get false false))))

(event EventBeginPlay
  (Input|EnableInput (Game|GetPlayerController (Variables|/Script/Engine.Pawn|GetPlayerState (Game|Player|GetPlayerPawn 0)))))

(event Input|KeyboardEvents|P
  (params (Key :type Key%20Structure :default "None"))
  (:Pressed
    (Development|PrintString "Hello")
    (Utilities|FlowControl|FlipFlop
      (:A
        (Variables|Default|SetRoation true))
      (:B
        (Variables|Default|SetRoation false)))))

(event Input|KeyboardEvents|G
  (params (Key :type Key%20Structure :default "None"))
  (:Pressed
    (Utilities|FlowControl|Sequence
      (:then_0
        (Variables|Default|SetInitialRotation (Transformation|GetWorldRotation (Variables|Default|GetCenterOfMass)))
        (Components|Animation|PlayAnimation (Variables|Default|GetSK_Mannequin) "/Game/Animation/StartingSequence.StartingSequence" false))
      (:then_1
        (Variables|Default|SetisStartingAnimPlayed? true)))))

(fn ConstructionScript)